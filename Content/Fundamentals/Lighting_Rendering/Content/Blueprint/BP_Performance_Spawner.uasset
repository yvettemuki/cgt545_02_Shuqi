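; Performance spawner actor that fills a configurable box with many copies of a static mesh or with point lights, apparently for stress-testing rendering cost.
; The construction script sizes the box, then adds components at random points inside it, looping on a count variable.
; A toggle switches from meshes to lights, which get random colors and optional shadow casting.
; Placement re-randomizes whenever construction reruns; the event graph is unused.
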(fn `UserConstructionScript`
  (bind _box (`self.Box`))
  (bind _returnvalue (`KismetMathLibrary.MakeTransform` (`KismetMathLibrary.RandomPointInBoundingBox` (`SceneComponent.RelativeLocation` _box) (`BoxComponent.BoxExtent` _box))))
  (`BoxComponent.SetBoxExtent` (`self.Box`) (`self.BoxSize`) false)
  (for _ (range (+ (`self.Number`) 1))
    (if (`self.SpawnsLightsInstead`)
      (bind _returnvalue_2 (`AddComponent|NODE_AddPointLightComponent-0` :`RelativeTransform` _returnvalue))
      (`LightComponentBase.SetCastShadows` _returnvalue_2 (`self.LightsHaveShadows`))
      (`LightComponent.SetLightColor` _returnvalue_2 (`KismetMathLibrary.MakeColor` (`KismetMathLibrary.RandomFloatInRange` 0.1 1.0) (`KismetMathLibrary.RandomFloatInRange` 0.1 1.0) (`KismetMathLibrary.RandomFloatInRange` 0.1 1.0)) true)
      (else
        (bind _returnvalue_3 (`AddComponent|NODE_AddStaticMeshComponent-0` :`RelativeTransform` _returnvalue))
        (`StaticMeshComponent.SetStaticMesh` _returnvalue_3 (`self.StaticMesh`))))))